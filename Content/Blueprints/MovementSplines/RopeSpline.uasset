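; Rope spline actor, filed under movement splines, that builds its visual representation in the construction script and has no runtime logic.
; It sets the spline's default world up vector from a variable, then optionally adds red arrows at each point along its up vector, left visible in game.
; An optional mesh pass adds spline mesh components between neighbouring points, matching their locations and tangents.
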(event EventBeginPlay)

(event Collision|EventActorBeginOverlap
  (params (OtherActor :type Actor%20Object%20Reference)))

(event EventTick
  (params (DeltaSeconds :type Float%20%28single-precision%29)))

(fn ConstructionScript
  (bind _spline (Variables|Default|GetSpline))
  (bind _spline_2 (Variables|Default|GetSpline))
  (Class|SplineComponent|SetDefaultUpVector (Variables|Default|GetSpline) (Variables|Default|GetUpVector) "World")
  (if (Variables|Default|GetCreate%20Arrows)
    (for _index (range 0 (Spline|GetNumberOfSplinePoints _spline))
      (bind _returnvalue (AddComponent|AddArrowComponent false (Math|Transform|MakeTransform (Math|Vector|MakeVector (.x (Spline|GetLocationatSplinePoint _spline _index "Local")) (.y (Spline|GetLocationatSplinePoint _spline _index "Local")) (.z (Spline|GetLocationatSplinePoint _spline _index "Local"))) (Math|Conversions|RotationFromXVector (Math|Vector|GetUpVector (Spline|GetRotationatSplinePoint _spline _index "Local"))) "2.500000,1,1.000000")))
      (Components|Arrow|SetArrowColor(LinearColor) _returnvalue (Utilities|Struct|MakeLinearColor 1.0 0.0 0.0 0.0))
      (Development|SetHiddeninGame _returnvalue false false)
      (if (Variables|Default|GetCreate%20Mesh)
        (for _index_2 (range 0 (- (Spline|GetNumberOfSplinePoints (Variables|Default|GetSpline)) 2))
          (bind _returnvalue_2 (AddComponent|AddSplineMeshComponent true))
          (Transformation|AttachComponentToComponent _returnvalue_2 (Variables|Default|GetDefaultSceneRoot) "None" "KeepRelative" "KeepRelative" "KeepRelative" true)
          (SplineMesh|SetStartandEnd _returnvalue_2 (.Location (Spline|GetLocationandTangentatSplinePoint _spline_2 _index_2 "Local")) (.Tangent (Spline|GetLocationandTangentatSplinePoint _spline_2 _index_2 "Local")) (.Location (Spline|GetLocationandTangentatSplinePoint _spline_2 (+ _index_2 1) "Local")) (.Tangent (Spline|GetLocationandTangentatSplinePoint _spline_2 (+ _index_2 1) "Local")) true :!class /Script/Engine.SplineMeshComponent))))
    (else
      (if (Variables|Default|GetCreate%20Mesh)
        (for _index_3 (range 0 (- (Spline|GetNumberOfSplinePoints (Variables|Default|GetSpline)) 2))
          (bind _returnvalue_3 (AddComponent|AddSplineMeshComponent true))
          (Transformation|AttachComponentToComponent _returnvalue_3 (Variables|Default|GetDefaultSceneRoot) "None" "KeepRelative" "KeepRelative" "KeepRelative" true)
          (SplineMesh|SetStartandEnd _returnvalue_3 (.Location (Spline|GetLocationandTangentatSplinePoint _spline_2 _index_3 "Local")) (.Tangent (Spline|GetLocationandTangentatSplinePoint _spline_2 _index_3 "Local")) (.Location (Spline|GetLocationandTangentatSplinePoint _spline_2 (+ _index_3 1) "Local")) (.Tangent (Spline|GetLocationandTangentatSplinePoint _spline_2 (+ _index_3 1) "Local")) true :!class /Script/Engine.SplineMeshComponent))))))